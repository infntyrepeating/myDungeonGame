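; BP_LobbyPlatform is a lobby platform that displays one player character model and tracks the PlayerController it belongs to.
; SpawnCharacter stores the controller, destroys any existing model, then spawns a BP_PlayerBaseModel at the PlayerSpawnTransform component's world transform.
; ClearCharacter releases the controller and destroys the current model, leaving the platform empty.
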(event `SpawnCharacter`
  (params (PlayerController :type "PlayerController Object Reference"))
  (bind _currentcharacter (`self.CurrentCharacter`))
  (set `self.PlayerController` PlayerController)
  (`/Engine/EditorBlueprintResources/StandardMacros.IsValid` _currentcharacter
    (:`Is Valid`
      (`self.K2_DestroyActor` _currentcharacter))
    (:`Is Not Valid`
      _))
  (bind _returnvalue (`|SpawnActorFromClass` "/Game/Blueprints/Lobby/BP_PlayerBaseModel.BP_PlayerBaseModel_C" (`SceneComponent.K2_GetComponentToWorld` (`self.PlayerSpawnTransform`)) "Undefined" "MultiplyWithRoot" null null))
  (set `self.CurrentCharacter` _returnvalue))

(event `ClearCharacter`
  (bind _currentcharacter (`self.CurrentCharacter`))
  (set `self.PlayerController` null)
  (`/Engine/EditorBlueprintResources/StandardMacros.IsValid` _currentcharacter
    (:`Is Valid`
      (`self.K2_DestroyActor` _currentcharacter)
      (set `self.CurrentCharacter` null))))

(fn `UserConstructionScript`)