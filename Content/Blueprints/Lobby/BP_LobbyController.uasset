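; Lobby player controller that shows the lobby UI and reports the player's info to the game mode.
; On BeginPlay, the local controller enables mouse input, creates WG_LobbyInterface and calls SetPlayerNameOnServer.
; That event and ToggleReadyStatusOnServer, which flips Ready in PlayerLobbyInfoPC, both pass the controller to BP_LobbyMode's UpdatePlayerInfo.
; A separate retry event repeats that update after a short delay.
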(event `tryAgainUpdatingLobbyInfo`
  (`KismetSystemLibrary.Delay` 0.1)
  (bind _asbp_lobby_mode (cast `/Game/Blueprints/Lobby/BP_LobbyMode` (`GameplayStatics.GetGameMode`)))
  (`/Game/Blueprints/Lobby/BP_LobbyMode.UpdatePlayerInfo` _asbp_lobby_mode self))

(event `self.ReceiveBeginPlay`
  (`self.SetUp`))

(event `SetPlayerNameOnServer`
  (bind _asbp_lobby_mode (cast `/Game/Blueprints/Lobby/BP_LobbyMode` (`GameplayStatics.GetGameMode`)))
  (`/Game/Blueprints/Lobby/BP_LobbyMode.UpdatePlayerInfo` _asbp_lobby_mode self))

(event `ToggleReadyStatusOnServer`
  (bind _playerlobbyinfopc (`self.PlayerLobbyInfoPC`))
  (setmembers `/Game/Blueprints/Lobby/S_LobbyPlayer` :`StructRef` _playerlobbyinfopc :`bReady` (not (`.bReady_8_D80AA174404ACBE1C22CBC841E0D98E6` (break `/Game/Blueprints/Lobby/S_LobbyPlayer` _playerlobbyinfopc))))
  (bind _asbp_lobby_mode (cast `/Game/Blueprints/Lobby/BP_LobbyMode` (`GameplayStatics.GetGameMode`)))
  (`/Game/Blueprints/Lobby/BP_LobbyMode.UpdatePlayerInfo` _asbp_lobby_mode self))

(fn `SetUp`
  (if (`self.IsLocalPlayerController`)
    (set `self.bShowMouseCursor` true)
    (`WidgetBlueprintLibrary.SetInputMode_GameAndUIEx` self null "DoNotLock" false)
    (bind _returnvalue (`|CreateWidget` "/Game/UI/Lobby/WG_LobbyInterface.WG_LobbyInterface_C"))
    (bind _output_get (set `self.LobbyUI_Ref` _returnvalue))
    (`UserWidget.AddToViewport` _output_get 0)
    (`self.SetPlayerNameOnServer`)))

(fn `UserConstructionScript`)