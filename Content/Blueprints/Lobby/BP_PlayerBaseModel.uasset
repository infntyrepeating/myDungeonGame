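; BP_PlayerBaseModel is a lobby player actor that displays a player's lobby info through its PlayerInfo widget component.
; UpdateLobbyInfo sets PlayerLobbyInfo, whose RepNotify passes the data to the WG_LobbyPlayer widget and makes the component visible.
; If the widget is not yet valid, the RepNotify retries itself on a short timer.
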(fn `OnRep_PlayerLobbyInfo`
  (bind _returnvalue (`WidgetComponent.GetWidget` (`self.Player Info`)))
  (`/Engine/EditorBlueprintResources/StandardMacros.IsValid` _returnvalue
    (:`Is Valid`
      (bind _aswg_lobby_player (cast `/Game/UI/Lobby/WG_LobbyPlayer` _returnvalue))
      (`/Game/UI/Lobby/WG_LobbyPlayer.Update` _aswg_lobby_player (`self.PlayerLobbyInfo`))
      (`SceneComponent.SetVisibility` (`self.Player Info`) true false))
    (:`Is Not Valid`
      (`KismetSystemLibrary.K2_SetTimer` null "OnRep_PlayerLobbyInfo" 0.1))))

(fn `UpdateLobbyInfo`
  (params (PlayerLobbyInfo :type "/Game/Blueprints/Lobby/S_LobbyPlayer Structure"))
  (set `self.PlayerLobbyInfo` PlayerLobbyInfo))

(fn `UserConstructionScript`)