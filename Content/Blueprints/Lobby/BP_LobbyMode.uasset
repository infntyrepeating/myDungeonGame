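; Lobby game mode that seats joining players on BP_LobbyPlatform actors and tracks who is ready.
; BeginPlay orders platforms by index tag; login and logout wait for that setup, then spawn characters on free platforms or clear vacated ones.
; UpdatePlayerInfo pushes name and ready state to the player's model, asking the controller to retry if unseated.
; It then writes joined, ready and all-ready status to player 0's lobby UI.
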(event `self.ReceiveBeginPlay`
  (`self.SetUpPlatforms`))

(event `self.K2_PostLogin`
  (params (NewPlayer :type "PlayerController Object Reference"))
  (`KismetArrayLibrary.Array_Add` (`self.PCs`) NewPlayer)
  (`self.ifPlatformsSetUpIsDone` :!label _label
    (:`true`
      (`self.UpdatePlatforms`))))

(event `self.K2_OnLogout`
  (params (ExitingController :type "Controller Object Reference"))
  (bind _asplayer_controller (cast `PlayerController` ExitingController))
  (`KismetArrayLibrary.Array_RemoveItem` (`self.PCs`) _asplayer_controller)
  (goto _label))

(fn `CheckIfEnoughPlayersReady`
  (locals (bAllPlayersReady :type Boolean))
  (set `local.bAllPlayersReady` true)
  (for _array_element (`self.PCs`)
    (bind _asbp_lobby_controller (cast `/Game/Blueprints/Lobby/BP_LobbyController` _array_element))
    (if (not (`.bReady_8_D80AA174404ACBE1C22CBC841E0D98E6` (break `/Game/Blueprints/Lobby/S_LobbyPlayer` (`/Game/Blueprints/Lobby/BP_LobbyController.PlayerLobbyInfoPC` _asbp_lobby_controller))))
      (set `local.bAllPlayersReady` false)))
  (bind _asbp_lobby_controller_2 (cast `/Game/Blueprints/Lobby/BP_LobbyController` (`GameplayStatics.GetPlayerController` 0)))
  (set `/Game/UI/Lobby/WG_LobbyInterface.bEnoughPeopleReady` (`local.bAllPlayersReady`) (`/Game/Blueprints/Lobby/BP_LobbyController.LobbyUI_Ref` _asbp_lobby_controller_2)))

(fn `CheckNumberOfPlayers`
  (locals (NumberOfPlayers :type Integer))
  (bind _pcs (`self.PCs`))
  (bind _asbp_lobby_controller (cast `/Game/Blueprints/Lobby/BP_LobbyController` (`GameplayStatics.GetPlayerController` 0)))
  (set `/Game/UI/Lobby/WG_LobbyInterface.JoinedPlayers` (`KismetArrayLibrary.Array_Length` _pcs) (`/Game/Blueprints/Lobby/BP_LobbyController.LobbyUI_Ref` _asbp_lobby_controller))
  (set `local.NumberOfPlayers` 0)
  (for _array_element _pcs
    (bind _asbp_lobby_controller_2 (cast `/Game/Blueprints/Lobby/BP_LobbyController` _array_element))
    (if (`.bReady_8_D80AA174404ACBE1C22CBC841E0D98E6` (break `/Game/Blueprints/Lobby/S_LobbyPlayer` (`/Game/Blueprints/Lobby/BP_LobbyController.PlayerLobbyInfoPC` _asbp_lobby_controller_2)))
      (set `local.NumberOfPlayers` (+ 1 (`local.NumberOfPlayers`)))))
  (bind _asbp_lobby_controller_3 (cast `/Game/Blueprints/Lobby/BP_LobbyController` (`GameplayStatics.GetPlayerController` 0)))
  (set `/Game/UI/Lobby/WG_LobbyInterface.ReadyPlayers` (`local.NumberOfPlayers`) (`/Game/Blueprints/Lobby/BP_LobbyController.LobbyUI_Ref` _asbp_lobby_controller_3)))

(fn `SetUpPlatforms`
  (bind _outactors (`GameplayStatics.GetAllActorsOfClass` "/Game/Blueprints/Lobby/BP_LobbyPlatform.BP_LobbyPlatform_C"))
  (for _index (range (+ (`KismetArrayLibrary.Array_LastIndex` _outactors) 1))
    (bind _outactors_2 (`GameplayStatics.GetAllActorsOfClassWithTag` "/Game/Blueprints/Lobby/BP_LobbyPlatform.BP_LobbyPlatform_C" (`KismetStringLibrary.Conv_StringToName` (`KismetStringLibrary.Conv_IntToString` _index))))
    (`KismetArrayLibrary.Array_Add` (`self.PlayerPlatforms`) (`|GetArrayItem` _outactors_2)))
  (set `self.bPlatformsSetUpDone` true))

(fn `UpdatePlatforms`
  (locals (Loop_PCAlreadyAdded :type Boolean))
  (for _array_element (`self.PCs`)
    (set `local.Loop_PCAlreadyAdded` false)
    (for _array_element_2 (`self.PlayerPlatforms`)
      (if (== (`/Game/Blueprints/Lobby/BP_LobbyPlatform.PlayerController` _array_element_2) _array_element)
        (set `local.Loop_PCAlreadyAdded` true)))
    (if (not (`local.Loop_PCAlreadyAdded`))
      (for _array_element_3 (`self.PlayerPlatforms`)
        (`/Engine/EditorBlueprintResources/StandardMacros.IsValid` (`/Game/Blueprints/Lobby/BP_LobbyPlatform.PlayerController` _array_element_3)
          (:`Is Not Valid`
            (`/Game/Blueprints/Lobby/BP_LobbyPlatform.SpawnCharacter` _array_element_3 _array_element)
            (break))))))
  (for _array_element_4 (`self.PlayerPlatforms`)
    (if (not (`KismetArrayLibrary.Array_Contains` (`self.PCs`) (`/Game/Blueprints/Lobby/BP_LobbyPlatform.PlayerController` _array_element_4)))
      (`/Game/Blueprints/Lobby/BP_LobbyPlatform.ClearCharacter` _array_element_4))))

(fn `UpdatePlayerInfo`
  (params (`Requesting PC` :type "PlayerController Object Reference"))
  (for _array_element (`self.PlayerPlatforms`)
    (if (== (`/Game/Blueprints/Lobby/BP_LobbyPlatform.PlayerController` _array_element) `Requesting PC`)
      (bind _asbp_player_base_model (cast `/Game/Blueprints/Lobby/BP_PlayerBaseModel` (`/Game/Blueprints/Lobby/BP_LobbyPlatform.CurrentCharacter` _array_element)))
      (`/Game/Blueprints/Lobby/BP_PlayerBaseModel.UpdateLobbyInfo` _asbp_player_base_model (make `/Game/Blueprints/Lobby/S_LobbyPlayer` `Requesting PC` (`KismetTextLibrary.Conv_StringToText` (`AdvancedSessionsLibrary.GetPlayerName` `Requesting PC`)) (`.bReady_8_D80AA174404ACBE1C22CBC841E0D98E6` (break `/Game/Blueprints/Lobby/S_LobbyPlayer` (`/Game/Blueprints/Lobby/BP_LobbyController.PlayerLobbyInfoPC` (cast `/Game/Blueprints/Lobby/BP_LobbyController` `Requesting PC` :!pure true)))) (`Controller.PlayerState` `Requesting PC`)))
      (`self.CheckIfEnoughPlayersReady`)
      (`self.CheckNumberOfPlayers`)
      (return)))
  (`/Game/Blueprints/Lobby/BP_LobbyController.tryAgainUpdatingLobbyInfo` (cast `/Game/Blueprints/Lobby/BP_LobbyController` `Requesting PC` :!pure true)))

(fn `UserConstructionScript`)