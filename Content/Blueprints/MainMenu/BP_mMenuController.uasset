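; Main menu controller Blueprint that builds the menu UI when play begins.
; BeginPlay adds the background and Start widgets to the viewport, then creates the Play menu without displaying it, keeping Start and Play references in variables.
; An unconnected "Starting Behaviour" chain duplicates the background and Start setup and holds the UI-only input mode and mouse cursor setup, so neither input setting runs.
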(event `self.ReceiveBeginPlay`
  (bind _returnvalue (`|CreateWidget` "/Game/UI/MainMenu/WG_MainMenuBackground.WG_MainMenuBackground_C"))
  (`UserWidget.AddToViewport` _returnvalue 0)
  (bind _returnvalue_2 (`|CreateWidget` "/Game/UI/MainMenu/WG_MainMenuStart.WG_MainMenuStart_C"))
  (bind _output_get (set `self.StartMenu` _returnvalue_2))
  (`UserWidget.AddToViewport` _output_get 0)
  (bind _returnvalue_3 (`|CreateWidget` "/Game/UI/MainMenu/WG_MainMenuPlay.WG_MainMenuPlay_C"))
  (set `self.PlayMenu` _returnvalue_3))

(fn `UserConstructionScript`)