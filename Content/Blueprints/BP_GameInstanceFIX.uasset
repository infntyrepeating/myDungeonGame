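; Game instance Blueprint holding helpers for level selection and dungeon room data.
; ShowLevelSelectmenu has an empty entry; its disconnected nodes would create or reuse the level-select widget, display it, and enable UI-only input with a cursor.
; FormatLevelName is built to cut a name at its first underscore, but its character-array conversion is not wired into the loop.
; GetRooms returns the stored DungeonRooms.
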(fn `FormatLevelName`
  (params (Input :type String))
  (returns (Output :type String))
  (locals (Element :type Integer))
  (for (_array_element _array_index) _
    (if (`KismetStringLibrary.EqualEqual_StrStr` _array_element "_")
      (set `local.Element` _array_index)
      (break)))
  (return (`KismetStringLibrary.GetSubstring` Input 0 (`local.Element`))))

(fn `GetRooms`
  (returns (Rooms :type "Array of DungeonStructure Structure"))
  (return (`self.Dungeon Rooms`)))

(fn `Show LevelSelectmenu`)