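; Player controller Blueprint that stores a player-selected level name and loads that level as a level instance near the player.
; GetlevelFromplayerselect passes the name to Test123, which saves it and sets IsReady; OnRep_isReady is empty.
; Instancelevel loads at an offset from the focal location, clears IsReady and widgets, restores game-only input and starts ambient sound.
; ClientEvent forwards to Multicast, which only increments and prints a debug counter.
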(event `ClientEvent`
  (params (NewParam :type Integer))
  (`self.Multicast` NewParam))

(event `Multicast`
  (params (NewParam :type Integer))
  (bind _result (`/Engine/EditorBlueprintResources/StandardMacros.IncrementInt` (`self.integer`))
    (:`  `
      (`KismetSystemLibrary.PrintString` (`KismetStringLibrary.Conv_IntToString` _result)))))

(event `Test123`
  (params (lvlname :type String))
  (set `self.Levelname` (`KismetTextLibrary.Conv_StringToText` lvlname))
  (set `self.isReady` true))

(event `Instance level`
  (params (levelname :type Text))
  (bind _returnvalue (`KismetTextLibrary.Conv_TextToString` levelname))
  (bind _output_get (set `self.Playerposition` (`self.GetFocalLocation`)))
  (bind _output_get_2 (set `self.NewVar` (50.0 10.0 0.0)))
  (`KismetSystemLibrary.PrintString` _returnvalue true true (struct :`G` 0.66 :`B` 1.0 :`A` 1.0) 20.0)
  (`LevelStreamingDynamic.LoadLevelInstance` _returnvalue (+ _output_get_2 _output_get) (struct) "" null)
  (set `self.isReady` false)
  (`WidgetLayoutLibrary.RemoveAllWidgets`)
  (`WidgetBlueprintLibrary.SetInputMode_GameOnly` (`GameplayStatics.GetPlayerController` 0))
  (`FMODBlueprintStatics.PlayEventAtLocation` "/Game/FMOD/Events/AmbientSound/AmbientSound.AmbientSound" (`self.GetLevelTransform`)))

(fn `GetlevelFromplayerselect`
  (params (Levelname :type Text))
  (bind _output_get (set `self.Levelname` Levelname))
  (`self.Test123` (`KismetTextLibrary.Conv_TextToString` _output_get)))

(fn `OnRep_isReady`)

(fn `UserConstructionScript`)