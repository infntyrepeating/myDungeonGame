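; Dungeon game state that waits for two players to be ready, then hands each the other's chosen level.
; Every Tick it polls both player controllers, inserting ready players' level names into an array and clearing readiness at the first unready one.
; When ready, it calls InstanceLevel on each controller with the swapped names.
; A separate LoadLevel function wraps level instance loading but is not called here.
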(event `self.ReceiveTick`
  (params (DeltaSeconds :type "Float (single-precision)"))
  (`self.playersReady`)
  (if (`self.Isready`)
    (for (_array_element _array_index) (`|MakeArray` 1 0)
      (bind _asbp_player_controler (cast `/Game/Blueprints/BP_PlayerControler` (`GameplayStatics.GetPlayerController` _array_index)))
      (`/Game/Blueprints/BP_PlayerControler.Instance level` _asbp_player_controler (`KismetTextLibrary.Conv_StringToText` (`|GetArrayItem` (`self.Levelname`) _array_element))))
    (set `self.Isready` false)))

(event `playersReady`
  (for (_array_element _array_index) (`|MakeArray` 0 1)
    (bind _asbp_player_controler (cast `/Game/Blueprints/BP_PlayerControler` (`GameplayStatics.GetPlayerController` _array_index)))
    (if (`/Game/Blueprints/BP_PlayerControler.isReady` _asbp_player_controler)
      (set `self.Isready` true)
      (bind _output_get (set `self.Levelname` (`self.Levelname`)))
      (`KismetSystemLibrary.PrintString` (`KismetStringLibrary.Conv_IntToString` _array_index) true true (struct :`G` 0.66 :`B` 1.0 :`A` 1.0) 20.0)
      (`KismetArrayLibrary.Array_Insert` _output_get (`KismetTextLibrary.Conv_TextToString` (`/Game/Blueprints/BP_PlayerControler.Levelname` _asbp_player_controler)) _array_element)
      (else
        (set `self.Isready` false)
        (break)))))

(fn `Load level`
  (params (playercontroller :type Integer) (Levelname :type Text))
  (`LevelStreamingDynamic.LoadLevelInstance` (`KismetTextLibrary.Conv_TextToString` Levelname) (0.0 0.0 0.0) (struct) "" null))

(fn `UserConstructionScript`)